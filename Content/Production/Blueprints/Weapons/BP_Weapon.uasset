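; BP_Weapon is a hitscan weapon that fires through its Shoot function, given an origin and direction.
; A CanShoot flag and FireDelay timer limit fire rate, with ShootTimerExpired re-enabling firing.
; Each shot runs a debug-drawn line trace over Range, ignoring the attach parent.
; Hits on Movable components receive an impulse scaled by Damage, while the hit actor takes fixed damage independent of that variable.
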(event Custom|ShootTimerExpired
  (Variables|Default|SetCanShoot true))

(event EventBeginPlay)

(event Collision|EventActorBeginOverlap
  (params (OtherActor :type Actor%20Object%20Reference)))

(event EventTick
  (params (DeltaSeconds :type Float%20%28single-precision%29)))

(fn ConstructionScript)

(fn Shoot
  (params (OriginLocation :type Vector) (ForwardVector :type Vector))
  (if (Variables|Default|GetCanShoot)
    (Variables|Default|SetCanShoot false)
    (Utilities|Time|SetTimerbyEvent (EventDispatchers|CreateEvent :!event Custom|ShootTimerExpired) (Variables|Default|GetFireDelay))
    (bind _outhit (Collision|LineTraceByChannel OriginLocation (+ OriginLocation (* ForwardVector (Variables|Default|GetRange))) "TraceTypeQuery3" false (Utilities|Array|MakeArray (Actor|GetAttachParentActor)) "ForDuration" true "(R=1.000000,G=0.000000,B=0.000000,A=1.000000)" "(R=0.000000,G=1.000000,B=0.000000,A=1.000000)" 1.0))
    (Utilities|IsValid (.hitcomponent _outhit)
      (:Is%20Valid
        (if (Utilities|Enum|Equal(Enum) (Variables|/Script/Engine.SceneComponent|GetMobility (.hitcomponent _outhit)) "Movable")
          (Physics|AddImpulseatLocation (.hitcomponent _outhit) (* ForwardVector (Variables|Default|GetDamage)) (.location _outhit) "None")
          (Game|Damage|ApplyDamage (.hitactor _outhit) 1e+01 0 0))))))