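; Shotgun weapon Blueprint that fires three BP_Projectile actors per shot.
; Shoot checks and clears CanShoot, starts a FireDelay timer, then spawns the projectiles along the given forward vector.
; Spawn points are the origin and two opposite fixed world-space offsets, all sharing one rotation, so the pellets fly parallel.
; An older hitscan path with damage and impulse remains disconnected, replaced by projectile impact.
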(event EventBeginPlay
  (|CallParentFunction) ; This node is disabled and will not be called.\nDrag off pins to build functionality.
)

(event Collision|EventActorBeginOverlap
  (params (OtherActor :type Actor%20Object%20Reference))
  (|CallParentFunction OtherActor) ; This node is disabled and will not be called.\nDrag off pins to build functionality.
)

(event EventTick
  (params (DeltaSeconds :type Float%20%28single-precision%29))
  (|CallParentFunction DeltaSeconds) ; This node is disabled and will not be called.\nDrag off pins to build functionality.
)

(fn ConstructionScript
  (|CallParentFunction))

(fn Shoot
  (params (OriginLocation :type Vector :default "0, 0, 0") (ForwardVector :type Vector :default "0, 0, 0"))
  (Variables|Default|SetRotator (Math|Conversions|RotationFromXVector ForwardVector))
  (Variables|Default|SetOrigin%20Location OriginLocation)
  (if (Variables|Default|GetCanShoot)
    (Variables|Default|SetCanShoot false)
    (Utilities|Time|SetTimerbyEvent (EventDispatchers|CreateEvent :!event ShootTimerExpired) (Variables|Default|GetFireDelay))
    (Game|SpawnActorfromClass "/Game/Production/Blueprints/Weapons/BP_Projectile.BP_Projectile_C" (Math|Transform|MakeTransform (Variables|Default|GetOrigin%20Location) (Variables|Default|GetRotator) "1.000000,1.000000,1.000000") "Undefined" "MultiplyWithRoot" 0 0)
    (Game|SpawnActorfromClass "/Game/Production/Blueprints/Weapons/BP_Projectile.BP_Projectile_C" (Math|Transform|MakeTransform (+ (Variables|Default|GetOrigin%20Location) "40.000000,0.000000,40.000000") (Variables|Default|GetRotator) "1.000000,1.000000,1.000000") "Undefined" "MultiplyWithRoot" 0 0)
    (Game|SpawnActorfromClass "/Game/Production/Blueprints/Weapons/BP_Projectile.BP_Projectile_C" (Math|Transform|MakeTransform (- (+ (Variables|Default|GetOrigin%20Location) "40.000000,0.000000,40.000000") "80.000000,0.000000,80.000000") (Variables|Default|GetRotator) "1.000000,1.000000,1.000000") "Undefined" "MultiplyWithRoot" 0 0)))