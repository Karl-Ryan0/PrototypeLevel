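; Assault rifle weapon Blueprint that fires projectiles at a limited rate.
; Shoot spawns a BP_Projectile at the given origin, oriented along the forward vector, whenever CanShoot is true.
; Each shot clears CanShoot and starts a FireDelay timer, with ShootTimerExpired re-enabling firing.
; An older hitscan path with line trace, damage and impulse remains disconnected, removed in favor of projectile impact.
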(event Custom|ShootTimerExpired
  (Variables|Default|SetCanShoot true))

(event EventBeginPlay)

(event Collision|EventActorBeginOverlap
  (params (OtherActor :type Actor%20Object%20Reference)))

(event EventTick
  (params (DeltaSeconds :type Float%20%28single-precision%29)))

(fn ConstructionScript)

(fn Shoot
  (params (OriginLocation :type Vector) (ForwardVector :type Vector))
  (if (Variables|Default|GetCanShoot)
    (Variables|Default|SetCanShoot false)
    (Utilities|Time|SetTimerbyEvent (EventDispatchers|CreateEvent :!event Custom|ShootTimerExpired) (Variables|Default|GetFireDelay))
    (Game|SpawnActorfromClass "/Game/Production/Blueprints/Weapons/BP_Projectile.BP_Projectile_C" (Math|Transform|MakeTransform OriginLocation (Math|Conversions|RotationFromXVector ForwardVector) "1.000000,1.000000,1.000000") "Undefined" "MultiplyWithRoot" 0 0)))