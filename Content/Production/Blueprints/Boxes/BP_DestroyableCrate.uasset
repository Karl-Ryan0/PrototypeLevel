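; BP_DestroyableCrate is a physics-simulated crate that takes damage on overlap and is destroyed when its health runs out.
; Any actor overlapping the Box trigger applies fixed damage to the crate, and overlapping BP_Projectile actors are then destroyed.
; BP_HealthComponent events print health changes and destroy the crate on depletion.
; Tick re-enables physics simulation on the Cube every frame.
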(event OnHealthChanged(BP_HealthComponent)
  (params (NewHealth :type Float%20%28double-precision%29))
  ;[0.15 0.15 0.15 0.5] Damage the actor
  (Development|PrintString (Utilities|String|Append "Current Box Health: " (Utilities|String|ToString(Float) NewHealth)) true true "(R=0.032573,G=1.000000,B=0.000000,A=1.000000)" 2.0 "Health"))

(event OnHealthDepleted(BP_HealthComponent)
  ;[0.15 0.15 0.15 0.5] Destroys object
  (Development|PrintString "BOX DESTROYED!!!")
  (Actor|DestroyActor))

(event OnComponentBeginOverlap(Box)
  (params (OverlappedComponent :type Primitive%20Component%20Object%20Reference) (OtherActor :type Actor%20Object%20Reference) (OtherComp :type Primitive%20Component%20Object%20Reference) (OtherBodyIndex :type Integer) (bFromSweep :type Boolean) (SweepResult :type Hit%20Result%20Structure%20%28by%20ref%29))
  ;[0.15 0.15 0.15 0.5] Applies damage and destroys the projectile
  (Game|Damage|ApplyDamage self 1e+01 0 0)
  (bind _asbp_projectile (Utilities|Casting|CastToBP_Projectile OtherActor))
  (Actor|DestroyActor _asbp_projectile))

(event EventTick
  (params (DeltaSeconds :type Float%20%28single-precision%29))
  (Physics|SetSimulatePhysics (Variables|Default|GetCube) true))

(fn ConstructionScript)