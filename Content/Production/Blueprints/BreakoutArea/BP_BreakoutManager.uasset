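; Manager for a breakout minigame that tracks how many target boxes remain and opens the way once all are destroyed.
; StartBreakout counts every BP_BreakoutBox in the level, and each BoxDestroyed call decrements that count, printing progress on screen.
; At zero it prints a win message, calls the BreakoutCompleted dispatcher and destroys all BP_VanishingDoor actors.
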(event Custom|StartBreakout
  (bind _outactors (Actor|GetAllActorsOfClass "/Game/Production/Blueprints/BreakoutArea/BP_BreakoutBox.BP_BreakoutBox_C"))
  (Development|PrintString (Utilities|String|Append "Targets Remaining: " (Utilities|String|ToString(Integer) (+ (Utilities|Array|Length _outactors) 0 0))))
  (Variables|Default|SetBoxesRemaining (+ (Utilities|Array|Length _outactors) 0 0)))

(event Custom|BoxDestroyed
  (bind _result (Math|Integer|DecrementInt (Variables|Default|GetBoxesRemaining))
    (:%20%20
      (bind _output_get (Variables|Default|SetBoxesRemaining _result))
      (if (== _output_get 0)
        (Development|PrintString "You win")
        (Default|CallBreakoutCompleted)
        (bind _outactors (Actor|GetAllActorsOfClass "/Game/Production/Blueprints/Doors/BP_VanishingDoor.BP_VanishingDoor_C"))
        (Actor|DestroyActor _outactors)
        (else
          (Development|PrintString (Utilities|String|Append "You have " (Utilities|String|ToString(Integer) (Variables|Default|GetBoxesRemaining)) " Targets Remaining") true true "(R=0.000000,G=0.000000,B=0.000000,A=1.000000)"))))))

(fn ConstructionScript)