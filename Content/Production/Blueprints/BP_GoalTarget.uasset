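; BP_GoalTarget is a goal trigger actor that rewards completion by spawning a key and a health shrine.
; Box overlaps increment and print a counter while it is below zero; otherwise a one-time guard lets it spawn BP_Key and BP_HealthShrine at hardcoded locations.
; It then destroys itself and runs GoalObjective, which broadcasts GoalCompleted.
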(event OnComponentBeginOverlap(Box)
  (params (OverlappedComponent :type Primitive%20Component%20Object%20Reference) (OtherActor :type Actor%20Object%20Reference) (OtherComp :type Primitive%20Component%20Object%20Reference) (OtherBodyIndex :type Integer) (bFromSweep :type Boolean) (SweepResult :type Hit%20Result%20Structure%20%28by%20ref%29))
  (if (< (Variables|Default|GetCount) 0)
    (Math|Integer|IncrementInt (Variables|Default|GetCount)
      (:%20%20
        (Development|PrintString (Utilities|String|ToString(Integer) (Variables|Default|GetCount)))))
    (elif (not (Variables|Default|GetKeySpawned))
      (Variables|Default|SetKeySpawned true)
      (Game|SpawnActorfromClass "/Game/Production/Blueprints/BP_Key.BP_Key_C" (Math|Transform|MakeTransform "-4800.000000,2159.000000,38.000000" "0, 0, 0" "1.000000,1.000000,1.000000") "Undefined" "MultiplyWithRoot" 0 0)
      (Game|SpawnActorfromClass "/Game/Production/Blueprints/Health/BP_HealthShrine.BP_HealthShrine_C" (Math|Transform|MakeTransform "-4800.000000,1159.000000,38.000000" "0, 0, 0" "1.000000,1.000000,1.000000") "Undefined" "MultiplyWithRoot" 0 0)
      (Actor|DestroyActor)
      (CallFunction|GoalObjective))))

(event Custom|Goal%20Objective
  (Default|CallGoalCompleted))

(event EventBeginPlay)

(event Collision|EventActorBeginOverlap
  (params (OtherActor :type Actor%20Object%20Reference)))

(event EventTick
  (params (DeltaSeconds :type Float%20%28single-precision%29)))

(fn ConstructionScript)