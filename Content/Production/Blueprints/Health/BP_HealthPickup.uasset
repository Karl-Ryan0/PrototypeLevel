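; BP_HealthPickup is a health pickup that heals the first-person shooter character when it overlaps the pickup's box.
; If the character's health component is below MaxHealth, it adds HealingAmount, caps the result at a hard-coded 100 rather than MaxHealth, prints the new health, and destroys itself.
; At full health the pickup stays in place and prints a message saying so.
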(event OnComponentBeginOverlap(Box)
  (params (OverlappedComponent :type Primitive%20Component%20Object%20Reference) (OtherActor :type Actor%20Object%20Reference) (OtherComp :type Primitive%20Component%20Object%20Reference) (OtherBodyIndex :type Integer) (bFromSweep :type Boolean) (SweepResult :type Hit%20Result%20Structure%20%28by%20ref%29))
  ;[0.15 0.15 0.15 0.5] Checks the character
  (bind _asbp_first_person_shooter_character (Utilities|Casting|CastToBP_FirstPersonShooterCharacter OtherActor))
  (Variables|Default|SetBP%20Health%20Component (Variables|/Game/Production/Blueprints/BP_FirstPersonShooterCharacter.BP_FirstPersonShooterCharacter_C|GetBP_HealthComponent _asbp_first_person_shooter_character))
  (if (< (Variables|/Game/Production/Blueprints/Health/BP_HealthComponent.BP_HealthComponent_C|GetHealth (Variables|/Game/Production/Blueprints/BP_FirstPersonShooterCharacter.BP_FirstPersonShooterCharacter_C|GetBP_HealthComponent _asbp_first_person_shooter_character)) (Variables|/Game/Production/Blueprints/Health/BP_HealthComponent.BP_HealthComponent_C|GetMaxHealth (Variables|/Game/Production/Blueprints/BP_FirstPersonShooterCharacter.BP_FirstPersonShooterCharacter_C|GetBP_HealthComponent _asbp_first_person_shooter_character)))
    (Variables|/Game/Production/Blueprints/Health/BP_HealthComponent.BP_HealthComponent_C|SetHealth (Variables|Default|GetBP%20Health%20Component) (+ (Variables|/Game/Production/Blueprints/Health/BP_HealthComponent.BP_HealthComponent_C|GetHealth (Variables|Default|GetBP%20Health%20Component)) (Variables|Default|GetHealingAmount)))
    (if (>= (Variables|/Game/Production/Blueprints/Health/BP_HealthComponent.BP_HealthComponent_C|GetHealth (Variables|Default|GetBP%20Health%20Component)) 1e+02)
      (Variables|/Game/Production/Blueprints/Health/BP_HealthComponent.BP_HealthComponent_C|SetHealth (Variables|Default|GetBP%20Health%20Component) 1e+02))
    (Development|PrintString (Utilities|String|Append "Current Health: " (Utilities|String|ToString(Float) (Variables|/Game/Production/Blueprints/Health/BP_HealthComponent.BP_HealthComponent_C|GetHealth (Variables|Default|GetBP%20Health%20Component)))) true true "(R=0.032573,G=1.000000,B=0.000000,A=1.000000)" 2.0 "Health")
    (Actor|DestroyActor)
    (else
      (Development|PrintString "Health is full" true true "(R=0.032573,G=1.000000,B=0.000000,A=1.000000)" 2.0 "Health"))))

(event EventBeginPlay)

(fn ConstructionScript)