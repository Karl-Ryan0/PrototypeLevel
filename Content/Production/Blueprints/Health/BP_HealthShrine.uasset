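; BP_HealthShrine is a healing shrine that restores the first-person shooter character's health when it sees the player.
; A PawnSensing sighting casts to the character and, after a short delay, adds HealingAmount to its BPHealthComponent while health is below maximum.
; The addition is not clamped, so health can exceed the maximum.
; A green on-screen print reports the current health or that it is full.
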(event OnSeePawn(PawnSensing)
  (params (Pawn :type Pawn%20Object%20Reference))
  (bind _asbp_first_person_shooter_character (Utilities|Casting|CastToBP_FirstPersonShooterCharacter Pawn))
  (Variables|Default|SetBP%20Health%20Component (Variables|/Game/Production/Blueprints/BP_FirstPersonShooterCharacter.BP_FirstPersonShooterCharacter_C|GetBP_HealthComponent _asbp_first_person_shooter_character))
  (Utilities|FlowControl|Delay 0.1)
  (if (< (Variables|/Game/Production/Blueprints/Health/BP_HealthComponent.BP_HealthComponent_C|GetHealth (Variables|Default|GetBP%20Health%20Component)) (Variables|/Game/Production/Blueprints/Health/BP_HealthComponent.BP_HealthComponent_C|GetMaxHealth (Variables|Default|GetBP%20Health%20Component)))
    (Variables|/Game/Production/Blueprints/Health/BP_HealthComponent.BP_HealthComponent_C|SetHealth (Variables|Default|GetBP%20Health%20Component) (+ (Variables|Default|GetHealingAmount) (Variables|/Game/Production/Blueprints/Health/BP_HealthComponent.BP_HealthComponent_C|GetHealth (Variables|Default|GetBP%20Health%20Component))))
    (Development|PrintString (Utilities|String|Append "Current Health: " (Utilities|String|ToString(Float) (Variables|/Game/Production/Blueprints/Health/BP_HealthComponent.BP_HealthComponent_C|GetHealth (Variables|Default|GetBP%20Health%20Component)))) true true "(R=0.032573,G=1.000000,B=0.000000,A=1.000000)" 2.0 "Health")
    (else
      (Development|PrintString "Health is full" true true "(R=0.032573,G=1.000000,B=0.000000,A=1.000000)" 2.0 "Health"))))

(fn ConstructionScript)