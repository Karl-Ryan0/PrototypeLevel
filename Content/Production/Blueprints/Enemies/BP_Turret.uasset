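; Enemy turret that aims and fires at the first-person player character whenever its PawnSensing component sees them.
; Each sighting interpolates toward the player, splitting rotation into actor yaw and clamped head pitch.
; It then fires the child-actor BP_TurretGun from the BulletStart transform.
; A health component prints health changes and destroys the turret on depletion.
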(event OnSeePawn(PawnSensing)
  (params (Pawn :type Pawn%20Object%20Reference))
  (bind _bulletstart (Variables|Default|GetBulletStart))
  (bind _asbp_first_person_shooter_character (Utilities|Casting|CastToBP_FirstPersonShooterCharacter Pawn))
  (CallFunction|ShootPlayer _asbp_first_person_shooter_character)
  (Default|Shoot (Variables|Default|GetGunBP) (Transformation|GetWorldLocation _bulletstart) (Math|Vector|GetForwardVector _bulletstart)))

(event OnHealthDepleted(BP_HealthComponent)
  (Development|PrintString "Turret Destroyed")
  (Actor|DestroyActor))

(event OnHealthChanged(BP_HealthComponent)
  (params (NewHealth :type Float%20%28double-precision%29))
  (Development|PrintString (Utilities|String|ToString(Float) NewHealth)))

(event EventBeginPlay
  (bind _asbp_turret_gun (Utilities|Casting|CastToBP_TurretGun (Variables|/Script/Engine.ChildActorComponent|GetChildActor (Variables|Default|GetGun))))
  (Variables|Default|SetGunBP _asbp_turret_gun))

(fn ConstructionScript)

(fn ShootPlayer
  (params (Player :type Actor%20Object%20Reference))
  (bind _returnvalue (Utilities|Time|GetWorldDeltaSeconds))
  (bind _returnvalue_2 (Transformation|GetActorLocation Player))
  (bind _head (Variables|Default|GetHead))
  (bind _rotationspeed (Variables|Default|GetRotationSpeed))
  (bind _head_2 (Variables|Default|GetHead))
  (bind _returnvalue_3 (Transformation|GetWorldRotation _head_2))
  (bind _returnvalue_4 (Transformation|GetWorldLocation _head))
  (bind _returnvalue_5 (Math|Rotator|FindLookatRotation _returnvalue_4 _returnvalue_2))
  (bind _returnvalue_6 (Math|Interpolation|RInterpTo _returnvalue_3 _returnvalue_5 _returnvalue _rotationspeed))
  (Transformation|SetRelativeRotation (Variables|Default|GetHead) (Math|Rotator|MakeRotator 0.0 (Math|Float|Clamp(Float) (.pitch _returnvalue_6) -2e+01 2e+01) 0.0) false false)
  (Transformation|SetActorRotation (Math|Rotator|MakeRotator 0.0 0.0 (.yaw _returnvalue_6))))