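; BP_Friendo is a wandering AI pawn that gives out an item the first time it sees another pawn.
; It loops AI moves to random reachable points around itself, pausing briefly after each successful arrival.
; On sighting a pawn while holding an item, it spawns that item nearby and zeroes its peripheral vision angle.
; Its health component prints health changes and destroys the actor on depletion.
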(event OnSeePawn(PawnSensing)
  (params (Pawn :type Pawn%20Object%20Reference))
  (if (Variables|Default|GetHas%20Item)
    (Variables|Default|SetHas%20Item false)
    (Game|SpawnActorfromClass (Variables|Default|GetSpawnedItem) (Math|Transform|MakeTransform (+ (Transformation|GetActorLocation) "50.000000,0.000000,10.000000") (Transformation|GetActorRotation) "1.000000,1.000000,1.000000") "Undefined" "MultiplyWithRoot" 0 0)
    (Class|PawnSensingComponent|SetPeripheralVisionAngle (Variables|Default|GetPawnSensing) 0.0)))

(event OnHealthDepleted(BP_HealthComponent)
  (Development|PrintString "Fren Destroyed   ) :")
  (Actor|DestroyActor))

(event OnHealthChanged(BP_HealthComponent)
  (params (NewHealth :type Float%20%28double-precision%29))
  (Development|PrintString (Utilities|String|ToString(Float) NewHealth)))

(event EventBeginPlay
  (AI|AIMoveTo self (.RandomLocation (AI|Navigation|GetRandomReachablePointinRadius (Transformation|GetActorLocation) 5e+03 0 0)) 0 5e+02 false :!label _label
    (:OnSuccess
      (Utilities|FlowControl|Delay 1.5)
      (goto _label))))

(fn ConstructionScript)