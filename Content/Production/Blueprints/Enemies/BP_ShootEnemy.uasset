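; Enemy pawn that chases and shoots the first-person shooter character when PawnSensing sees it.
; Each sighting starts an AI move toward the player and immediately fires the child-actor weapon from ShootPoint, without waiting for arrival.
; The health component logs changes and destroys the enemy on depletion.
; ShootPlayer interpolates aim with clamped ShootPoint pitch and actor yaw, but nothing here calls it.
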(event OnSeePawn(PawnSensing)
  (params (Pawn :type Pawn%20Object%20Reference))
  (bind _shootpoint (Variables|Default|GetShootPoint))
  (bind _asbp_first_person_shooter_character (Utilities|Casting|CastToBP_FirstPersonShooterCharacter Pawn))
  (AI|AIMoveTo self "0, 0, 0" _asbp_first_person_shooter_character 5.0 false
    (:then
      (Default|Shoot (Variables|Default|GetWeaponBP) (Transformation|GetWorldLocation _shootpoint) (Math|Vector|GetForwardVector _shootpoint)))))

(event OnHealthDepleted(BP_HealthComponent)
  (Development|PrintString "Pawn Destroyed")
  (Actor|DestroyActor))

(event OnHealthChanged(BP_HealthComponent)
  (params (NewHealth :type Float%20%28double-precision%29))
  (Development|PrintString (Utilities|String|ToString(Float) NewHealth)))

(event EventBeginPlay
  (Variables|Default|SetOriginLocation (Transformation|GetActorLocation))
  (Variables|Default|SetOriginRotation (Transformation|GetActorRotation))
  (bind _asbp_weapon (Utilities|Casting|CastToBP_Weapon (Variables|/Script/Engine.ChildActorComponent|GetChildActor (Variables|Default|GetGun))))
  (Variables|Default|SetWeaponBP _asbp_weapon))

(fn ConstructionScript)

(fn ShootPlayer
  (params (Player :type Actor%20Object%20Reference))
  (bind _returnvalue (Utilities|Time|GetWorldDeltaSeconds))
  (bind _returnvalue_2 (Transformation|GetActorLocation Player))
  (bind _rotationspeed (Variables|Default|GetRotationSpeed))
  (bind _shootpoint (Variables|Default|GetShootPoint))
  (bind _shootpoint_2 (Variables|Default|GetShootPoint))
  (bind _returnvalue_3 (Transformation|GetWorldRotation _shootpoint_2))
  (bind _returnvalue_4 (Transformation|GetWorldLocation _shootpoint))
  (bind _returnvalue_5 (Math|Rotator|FindLookatRotation _returnvalue_4 _returnvalue_2))
  (bind _returnvalue_6 (Math|Interpolation|RInterpTo _returnvalue_3 _returnvalue_5 _returnvalue _rotationspeed))
  (Transformation|SetRelativeRotation (Variables|Default|GetShootPoint) (Math|Rotator|MakeRotator 0.0 (Math|Float|Clamp(Float) (.pitch _returnvalue_6) -2e+01 2e+01) 0.0) false false)
  (Transformation|SetActorRotation (Math|Rotator|MakeRotator 0.0 0.0 (.yaw _returnvalue_6))))