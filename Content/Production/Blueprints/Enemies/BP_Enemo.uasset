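; BP_Enemo is an enemy that roams the level and drops a key when killed.
; On BeginPlay it moves via AIMoveTo to random reachable points around itself, picking a new one after each successful arrival; failed moves are not retried.
; Its health component prints health changes, and on depletion it calls the destroyed-objective event, destroys itself and spawns BP_Key at its location.
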(event OnHealthDepleted(BP_HealthComponent)
  (Default|CallDestroyedObjective)
  (Actor|DestroyActor)
  (Game|SpawnActorfromClass "/Game/Production/Blueprints/BP_Key.BP_Key_C" (Math|Transform|MakeTransform (Transformation|GetActorLocation) "0, 0, 0" "1.000000,1.000000,1.000000") "Undefined" "MultiplyWithRoot" 0 0))

(event OnHealthChanged(BP_HealthComponent)
  (params (NewHealth :type Float%20%28double-precision%29))
  (Development|PrintString (Utilities|String|ToString(Float) NewHealth)))

(event EventBeginPlay
  (AI|AIMoveTo self (.RandomLocation (AI|Navigation|GetRandomReachablePointinRadius (Transformation|GetActorLocation) 5e+03 0 0)) 0 5e+02 false :!label _label
    (:OnSuccess
      (Utilities|FlowControl|Delay 0.0)
      (goto _label))))

(fn ConstructionScript
  (|CallParentFunction))