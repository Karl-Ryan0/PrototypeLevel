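; Enemy cannon that tracks a player seen through pawn sensing and fires cannonballs.
; On each sighting, ShootPlayer smoothly aims at the player, splitting rotation into actor yaw and clamped head pitch.
; A CanShoot flag gates spawning BP_Cannonball at the Arrow's transform.
; Re-arming relies on a later sighting starting a five-second delay, rather than starting at the shot.
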(event OnSeePawn(PawnSensing)
  (params (Pawn :type Pawn%20Object%20Reference))
  (bind _arrow (Variables|Default|GetArrow))
  (bind _asbp_first_person_shooter_character (Utilities|Casting|CastToBP_FirstPersonShooterCharacter Pawn))
  (CallFunction|ShootPlayer _asbp_first_person_shooter_character)
  (if (Variables|Default|GetCanShoot)
    (Variables|Default|SetCanShoot false)
    (Development|PrintString "Hello")
    (Game|SpawnActorfromClass "/Game/Production/Blueprints/Enemies/BP_Cannonball.BP_Cannonball_C" (Math|Transform|MakeTransform (Transformation|GetWorldLocation _arrow) (Transformation|GetWorldRotation _arrow) "1.000000,1.000000,1.000000") "AlwaysSpawn" "MultiplyWithRoot" 0 0)
    (else
      (Utilities|FlowControl|Delay 5.0)
      (Variables|Default|SetCanShoot true))))

(fn ConstructionScript)

(fn ShootPlayer
  (params (Player :type Actor%20Object%20Reference))
  (bind _returnvalue (Utilities|Time|GetWorldDeltaSeconds))
  (bind _returnvalue_2 (Transformation|GetActorLocation Player))
  (bind _head (Variables|Default|GetHead))
  (bind _rotationspeed (Variables|Default|GetRotationSpeed))
  (bind _head_2 (Variables|Default|GetHead))
  (bind _returnvalue_3 (Transformation|GetWorldRotation _head_2))
  (bind _returnvalue_4 (Transformation|GetWorldLocation _head))
  (bind _returnvalue_5 (Math|Rotator|FindLookatRotation _returnvalue_4 _returnvalue_2))
  (bind _returnvalue_6 (Math|Interpolation|RInterpTo _returnvalue_3 _returnvalue_5 _returnvalue _rotationspeed))
  (Transformation|SetRelativeRotation (Variables|Default|GetHead) (Math|Rotator|MakeRotator 0.0 (Math|Float|Clamp(Float) (.pitch _returnvalue_6) -2e+01 2e+01) 0.0) false false)
  (Transformation|SetActorRotation (Math|Rotator|MakeRotator 0.0 0.0 (.yaw _returnvalue_6))))