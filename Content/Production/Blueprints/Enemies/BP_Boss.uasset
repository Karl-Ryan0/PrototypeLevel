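; BP_Boss is an enemy boss that chases and shoots the first-person player and spins in place on Tick while ShouldRotate is set.
; AI perception updates stop the spin, start a move toward the player and immediately fire its child-actor weapon from ShootPoint.
; Forgetting a target sends it back to its spawn location and re-enables spinning as that move begins.
; Its health component prints health changes and destroys it on depletion.
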(event OnTargetPerceptionUpdated(AIPerception)
  (params (Actor :type Actor%20Object%20Reference) (Stimulus :type AI%20Stimulus%20Structure))
  (bind _shootpoint (Variables|Default|GetShootPoint))
  (Variables|Default|SetShouldRotate false)
  (bind _asbp_first_person_shooter_character (Utilities|Casting|CastToBP_FirstPersonShooterCharacter Actor))
  (AI|AIMoveTo self "0, 0, 0" _asbp_first_person_shooter_character 3e+02 false
    (:then
      (Default|Shoot (Variables|Default|GetWeaponBP) (Transformation|GetWorldLocation _shootpoint) (Math|Vector|GetForwardVector _shootpoint)))))

(event OnTargetPerceptionForgotten(AIPerception)
  (params (Actor :type Actor%20Object%20Reference))
  (AI|AIMoveTo self (Variables|Default|GetSpawnLocation) 0 0.0 false
    (:then
      (Variables|Default|SetShouldRotate true))))

(event OnHealthDepleted(BP_HealthComponent)
  (Development|PrintString "Boss Destroyed")
  (Actor|DestroyActor))

(event OnHealthChanged(BP_HealthComponent)
  (params (NewHealth :type Float%20%28double-precision%29))
  (Development|PrintString (Utilities|String|ToString(Float) NewHealth)))

(event EventBeginPlay
  (Variables|Default|SetSpawnLocation (Transformation|GetActorLocation self))
  (bind _asbp_weapon (Utilities|Casting|CastToBP_Weapon (Variables|/Script/Engine.ChildActorComponent|GetChildActor (Variables|Default|GetGun))))
  (Variables|Default|SetWeaponBP _asbp_weapon))

(event EventTick
  (params (DeltaSeconds :type Float%20%28single-precision%29))
  (if (Variables|Default|GetShouldRotate)
    (Transformation|AddActorLocalRotation (Math|Rotator|MakeRotator 0.0 0.0 (* DeltaSeconds 3e+01)) false false)))

(fn ConstructionScript)