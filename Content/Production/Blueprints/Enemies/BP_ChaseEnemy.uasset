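; BP_ChaseEnemy is an enemy that chases the first-person player character once PawnSensing spots it.
; It uses AI MoveTo to reach the player, applies damage on success, then either teleports back to its spawn transform or destroys itself, depending on ShouldRespawn.
; A health component drives death, destroying the enemy when health is depleted, with debug prints for health changes and destruction.
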(event OnSeePawn(PawnSensing)
  (params (Pawn :type Pawn%20Object%20Reference))
  (bind _asbp_first_person_shooter_character (Utilities|Casting|CastToBP_FirstPersonShooterCharacter Pawn))
  (AI|AIMoveTo self "0, 0, 0" _asbp_first_person_shooter_character 5.0 false
    (:OnSuccess
      (Game|Damage|ApplyDamage _asbp_first_person_shooter_character 1.0 0 0)
      (if (Variables|Default|GetShouldRespawn)
        (Transformation|Teleport (Variables|Default|GetOriginLocation) (Variables|Default|GetOriginRotation))
        (else
          (Actor|DestroyActor))))))

(event OnHealthDepleted(BP_HealthComponent)
  (Development|PrintString "Pawn Destroyed")
  (Actor|DestroyActor))

(event OnHealthChanged(BP_HealthComponent)
  (params (NewHealth :type Float%20%28double-precision%29))
  (Development|PrintString (Utilities|String|ToString(Float) NewHealth)))

(event EventBeginPlay
  (Variables|Default|SetOriginLocation (Transformation|GetActorLocation))
  (Variables|Default|SetOriginRotation (Transformation|GetActorRotation)))

(fn ConstructionScript)