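; Objective manager actor that runs a fixed sequence of objective actors, revealing them one after another.
; On BeginPlay it hides every entry in OrderedObjectives, then makes the first current.
; SetCurrentObjective unhides the objective, prints its instructions and binds to its completion event.
; Completion increments the index and activates the next valid objective; completed objectives are not re-hidden here.
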(event Custom|OnEventCompleted
  (bind _result (Math|Integer|IncrementInt (Variables|Default|GetCurrentObjectiveIndex))
    (:%20%20
      (Utilities|IsValid (Utilities|Array|Get(acopy) (Variables|Default|GetOrderedObjectives) _result)
        (:Is%20Valid
          (CallFunction|SetCurrentObjective (Utilities|Array|Get(acopy) (Variables|Default|GetOrderedObjectives) _result)))))))

(event EventBeginPlay
  (if (Utilities|Array|IsNotEmpty (Variables|Default|GetOrderedObjectives))
    (for _array_element (Variables|Default|GetOrderedObjectives)
      (Rendering|SetActorHiddenInGame _array_element true))
    (CallFunction|SetCurrentObjective (Utilities|Array|Get(acopy) (Variables|Default|GetOrderedObjectives)))))

(fn ConstructionScript)

(fn SetCurrentObjective
  (params (NewObjective :type BP%20Objective%20Marker%20Object%20Reference))
  (Rendering|SetActorHiddenInGame NewObjective false)
  (Development|PrintString (Variables|/Game/Production/Blueprints/Objectives/BP_ObjectiveMarker.BP_ObjectiveMarker_C|GetInstructions NewObjective))
  (EventDispatchers|BindEventtoCompleted NewObjective (EventDispatchers|CreateEvent :!event Custom|OnEventCompleted)))