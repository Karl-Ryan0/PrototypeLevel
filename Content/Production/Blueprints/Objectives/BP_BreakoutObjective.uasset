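; BP_BreakoutObjective is an objective that completes when the Breakout minigame is finished.
; On BeginPlay it binds BreakoutFinished to the completion event of its BPBreakoutManager reference, if that reference is valid.
; BreakoutFinished fires the Completed dispatcher, destroys the objective, prints a debug message and destroys all BP_Paddle actors.
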(event Custom|BreakoutFinished
  (Default|CallCompleted)
  (Actor|DestroyActor)
  (Development|PrintString "BREAKOUT COMPLETED!!!!!")
  (bind _outactors (Actor|GetAllActorsOfClass "/Game/Production/Blueprints/BreakoutArea/BP_Paddle.BP_Paddle_C"))
  (Actor|DestroyActor _outactors))

(event EventBeginPlay
  (bind _bp_breakoutmanager (Variables|Default|GetBP_BreakoutManager))
  (|CallParentFunction)
  (Utilities|IsValid _bp_breakoutmanager
    (:Is%20Valid
      (EventDispatchers|BindEventtoBreakoutCompleted _bp_breakoutmanager (delegate Custom|BreakoutFinished)))))

(fn ConstructionScript
  (|CallParentFunction))