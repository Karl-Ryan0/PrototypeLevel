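; BP_EnemyKillObjective is an objective that completes when a referenced enemy is killed and updates the player's checkpoint.
; On BeginPlay it binds OnEnemyKilled to that enemy's destroyed-objective event, provided the reference is valid.
; When the event fires, it signals completion, destroys itself, prints a message and copies CheckpointLocation into the first-person shooter character's RespawnLocation.
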(event Custom|OnEnemyKilled
  (Default|CallCompleted)
  (Actor|DestroyActor)
  (Development|PrintString "Objective Completed")
  (bind _asbp_first_person_shooter_character (Utilities|Casting|CastToBP_FirstPersonShooterCharacter (Game|GetPlayerCharacter 0)))
  (Variables|/Game/Production/Blueprints/BP_FirstPersonShooterCharacter.BP_FirstPersonShooterCharacter_C|SetRespawnLocation _asbp_first_person_shooter_character (Variables|Default|GetCheckpointLocation)))

(event EventBeginPlay
  (bind _enemy_ref (Variables|Default|GetEnemy%20Ref))
  (|CallParentFunction)
  (Utilities|IsValid _enemy_ref
    (:Is%20Valid
      (EventDispatchers|BindEventtoDestroyedObjective _enemy_ref (delegate Custom|OnEnemyKilled)))))

(fn ConstructionScript
  (|CallParentFunction))