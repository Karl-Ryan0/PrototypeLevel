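; BP_FootballObjective is an objective actor that completes when its referenced football goal reports completion.
; On BeginPlay it binds to GoalRef's completion event, printing a placeholder "Hello" if the reference is invalid.
; On completion it calls Completed, destroys itself, prints a message and sets the player character's respawn location to CheckpointLocation.
; An identical door-unlock handler exists, but its binding to DoorRef is disconnected and never runs.
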(event Custom|OnGoalCompleted
  (Default|CallCompleted)
  (Actor|DestroyActor)
  (Development|PrintString "Objective Completed")
  (bind _asbp_first_person_shooter_character (Utilities|Casting|CastToBP_FirstPersonShooterCharacter (Game|GetPlayerCharacter 0)))
  (Variables|/Game/Production/Blueprints/BP_FirstPersonShooterCharacter.BP_FirstPersonShooterCharacter_C|SetRespawnLocation _asbp_first_person_shooter_character (Variables|Default|GetCheckpointLocation)))

(event Custom|OnDoorUnlocked
  (Default|CallCompleted)
  (Actor|DestroyActor)
  (Development|PrintString "Objective Completed")
  (bind _asbp_first_person_shooter_character (Utilities|Casting|CastToBP_FirstPersonShooterCharacter (Game|GetPlayerCharacter 0)))
  (Variables|/Game/Production/Blueprints/BP_FirstPersonShooterCharacter.BP_FirstPersonShooterCharacter_C|SetRespawnLocation _asbp_first_person_shooter_character (Variables|Default|GetCheckpointLocation)))

(event EventBeginPlay
  (bind _goalref (Variables|Default|GetGoalRef))
  (|CallParentFunction)
  (Utilities|IsValid _goalref
    (:Is%20Valid
      (EventDispatchers|BindEventtoGoalCompleted _goalref (delegate Custom|OnGoalCompleted)))
    (:Is%20Not%20Valid
      (Development|PrintString "Hello"))))

(fn ConstructionScript
  (|CallParentFunction))