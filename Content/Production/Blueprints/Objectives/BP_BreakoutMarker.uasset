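; BP_BreakoutMarker is an objective marker actor that completes when a breakout finishes.
; On BeginPlay it binds to the BreakoutCompleted event of its referenced breakout manager, printing a placeholder debug string if that reference is invalid.
; When the event fires, it calls its Completed dispatcher, destroys itself and prints a debug message.
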(event Custom|BreakoutFinished
  (Default|CallCompleted)
  (Actor|DestroyActor)
  (Development|PrintString "BREAKOUT COMPLETED!!!!!"))

(event EventBeginPlay
  (bind _bp_breakoutmanager (Variables|Default|GetBP_BreakoutManager))
  (|CallParentFunction)
  (Utilities|IsValid _bp_breakoutmanager
    (:Is%20Valid
      (EventDispatchers|BindEventtoBreakoutCompleted _bp_breakoutmanager (delegate Custom|BreakoutFinished)))
    (:Is%20Not%20Valid
      (Development|PrintString "Hello"))))

(fn ConstructionScript
  (|CallParentFunction))