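; BP_TargetManager tracks how many shooting targets remain in the level and ends the game when all are destroyed.
; On BeginPlay it sums all static, floating and moving target actors into TargetsRemaining and prints the count.
; Its TargetDestroyed event decrements that count, printing the remainder or, at zero, a win message before quitting after a short delay.
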(event Custom|TargetDestroyed
  (bind _result (Math|Integer|DecrementInt (Variables|Default|GetTargetsRemaining))
    (:%20%20
      (bind _output_get (Variables|Default|SetTargetsRemaining _result))
      (if (== _output_get 0)
        (Development|PrintString "You win")
        (Utilities|FlowControl|Delay 4.0)
        (Game|QuitGame 0 "Quit" false)
        (else
          (Development|PrintString (Utilities|String|Append "You have " (Utilities|String|ToString(Integer) (Variables|Default|GetTargetsRemaining)) " Targets Remaining") true true "(R=0.000000,G=0.000000,B=0.000000,A=1.000000)"))))))

(event EventBeginPlay
  (bind _outactors (Actor|GetAllActorsOfClass "/Game/Production/Blueprints/Targets/BP_StaticTarget.BP_StaticTarget_C"))
  (bind _outactors_2 (Actor|GetAllActorsOfClass "/Game/Production/Blueprints/Targets/BP_FloatingTarget.BP_FloatingTarget_C"))
  (bind _outactors_3 (Actor|GetAllActorsOfClass "/Game/Production/Blueprints/Targets/BP_MovingTarget.BP_MovingTarget_C"))
  (Development|PrintString (Utilities|String|Append "Targets Remaining: " (Utilities|String|ToString(Integer) (+ (Utilities|Array|Length _outactors_3) (Utilities|Array|Length _outactors_2) (Utilities|Array|Length _outactors)))))
  (Variables|Default|SetTargetsRemaining (+ (Utilities|Array|Length _outactors_3) (Utilities|Array|Length _outactors_2) (Utilities|Array|Length _outactors))))

(fn ConstructionScript)