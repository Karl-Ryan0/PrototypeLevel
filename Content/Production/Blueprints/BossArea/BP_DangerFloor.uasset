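; BP_DangerFloor is a boss-area floor hazard that damages overlapping actors after its switch event fires three times.
; FlipTheSwitch advances three boolean latches; the third waits briefly, swaps the floor material and applies damage once to everything overlapping the mesh.
; After another delay, Reset clears the latches, restores the material, and ResetButtons is called on all BP_BossPlate actors.
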(event Custom|FlipTheSwitch
  (if (Variables|Default|GetSwitch1)
    (if (Variables|Default|GetSwitch2)
      (if (not (Variables|Default|GetSwitch3))
        (Variables|Default|SetSwitch3 true)
        (Utilities|FlowControl|Delay 3.0)
        (Rendering|Material|SetMaterial (Variables|Default|GetSM_DangerFloor) 0 "/MeshModelingToolsetExp/Materials/GizmoDefaultMaterial.GizmoDefaultMaterial")
        (for _array_element (Collision|GetOverlappingActors (Variables|Default|GetSM_DangerFloor) 0 :!class /Script/Engine.PrimitiveComponent)
          (Game|Damage|ApplyDamage _array_element (Variables|Default|GetDamageAmount) 0 0))
        (Utilities|FlowControl|Delay 2.0)
        (CallFunction|Reset)
        (bind _outactors (Actor|GetAllActorsOfClass "/Game/Production/Blueprints/BossArea/BP_BossPlate.BP_BossPlate_C"))
        (Default|ResetButtons _outactors))
      (else
        (Variables|Default|SetSwitch2 true)))
    (else
      (Variables|Default|SetSwitch1 true))))

(fn ConstructionScript)

(fn Reset
  (Variables|Default|SetSwitch1 false)
  (Variables|Default|SetSwitch2 false)
  (Variables|Default|SetSwitch3 false)
  (Rendering|Material|SetMaterial (Variables|Default|GetSM_DangerFloor) 0 "/DatasmithContent/Materials/C4DReference.C4DReference"))