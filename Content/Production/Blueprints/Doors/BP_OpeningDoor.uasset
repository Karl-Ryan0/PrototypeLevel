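; BP_OpeningDoor is a door Blueprint that responds to open and close events from its parent class.
; Opening calls DoorObjective, then instantly offsets the Cube and rotates the root component to an open pose, with no animated transition.
; Closing only runs when ShouldClose is set, waiting a short delay before snapping both components back to their closed transforms.
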(event EventOpenDoor
  ;[0.15 0.15 0.15 0.5] Responding to events from the parent class
  (CallFunction|DoorObjective)
  (Transformation|SetRelativeLocation (Variables|Default|GetCube) "70.000000,50.000000,100.000000" false false)
  (Transformation|SetRelativeRotation (Variables|Default|GetDefaultSceneRoot) "0.000000,270.000000,0.000000" false false))

(event EventCloseDoor
  ;[0.15 0.15 0.15 0.5] Responding to events from the parent class
  (if (Variables|Default|GetShouldClose)
    (Utilities|FlowControl|Delay 3.0)
    (Transformation|SetRelativeLocation (Variables|Default|GetCube) "0.000000,0.000000,100.000000" false false)
    (Transformation|SetRelativeRotation (Variables|Default|GetDefaultSceneRoot) "0, 0, 0" false false)))

(fn ConstructionScript
  (|CallParentFunction))