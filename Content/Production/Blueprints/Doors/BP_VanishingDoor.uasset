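; Door Blueprint that opens by vanishing rather than moving, child of a parent whose construction script it calls.
; OpenDoor calls DoorObjective, then hides the actor and disables its collision.
; CloseDoor acts only when ShouldClose is set, restoring visibility and collision after a fixed delay.
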(event EventOpenDoor
  (CallFunction|DoorObjective)
  (Rendering|SetActorHiddenInGame true)
  (Collision|SetActorEnableCollision false))

(event EventCloseDoor
  (if (Variables|Default|GetShouldClose)
    (Utilities|FlowControl|Delay 3.0)
    (Rendering|SetActorHiddenInGame false)
    (Collision|SetActorEnableCollision true)))

(fn ConstructionScript
  (|CallParentFunction))