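; BP_GoalTarget is a goal trigger in the football area that rewards the third overlap of its Box component.
; The first two overlaps increment and print a counter, with no check on what entered.
; The third spawns a BP_HealthShrine at a hardcoded location, destroys the target, broadcasts GoalCompleted through GoalObjective and destroys all BPDestroyingDoor actors.
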(event OnComponentBeginOverlap(Box)
  (params (OverlappedComponent :type Primitive%20Component%20Object%20Reference) (OtherActor :type Actor%20Object%20Reference) (OtherComp :type Primitive%20Component%20Object%20Reference) (OtherBodyIndex :type Integer) (bFromSweep :type Boolean) (SweepResult :type Hit%20Result%20Structure%20%28by%20ref%29))
  (if (< (Variables|Default|GetCount) 2)
    (Math|Integer|IncrementInt (Variables|Default|GetCount)
      (:%20%20
        (Development|PrintString (Utilities|String|ToString(Integer) (Variables|Default|GetCount)))))
    (else
      (Game|SpawnActorfromClass "/Game/Production/Blueprints/Health/BP_HealthShrine.BP_HealthShrine_C" (Math|Transform|MakeTransform "-4800.000000,1159.000000,38.000000" "0, 0, 0" "1.000000,1.000000,1.000000") "Undefined" "MultiplyWithRoot" 0 0)
      (Actor|DestroyActor)
      (CallFunction|GoalObjective)
      (bind _outactors (Actor|GetAllActorsOfClass "/Game/Production/Blueprints/Doors/BPDestroyingDoor.BPDestroyingDoor_C"))
      (Actor|DestroyActor _outactors))))

(event Custom|Goal%20Objective
  (Default|CallGoalCompleted))

(event EventBeginPlay)

(event Collision|EventActorBeginOverlap
  (params (OtherActor :type Actor%20Object%20Reference)))

(event EventTick
  (params (DeltaSeconds :type Float%20%28single-precision%29)))

(fn ConstructionScript)