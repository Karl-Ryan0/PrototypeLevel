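; BP_AmmoPickup is a respawning pickup that gives the first-person shooter character extra reserve ammo.
; On overlap with that character it adds AmmoAmount to ReserveAmmo, with no clamp to FullAmmo, and prints both values as a debug string.
; It then hides itself and disables collision for a short delay before reappearing, so the same actor is reused instead of destroyed.
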(event Collision|EventActorBeginOverlap
  (params (OtherActor :type Actor%20Object%20Reference))
  (bind _asbp_first_person_shooter_character (Utilities|Casting|CastToBP_FirstPersonShooterCharacter OtherActor))
  (bind _output_get (Variables|/Game/Production/Blueprints/BP_FirstPersonShooterCharacter.BP_FirstPersonShooterCharacter_C|SetReserveAmmo _asbp_first_person_shooter_character (+ (Variables|/Game/Production/Blueprints/BP_FirstPersonShooterCharacter.BP_FirstPersonShooterCharacter_C|GetReserveAmmo _asbp_first_person_shooter_character) (Variables|Default|GetAmmoAmount))))
  (Rendering|SetActorHiddenInGame true)
  (Collision|SetActorEnableCollision false)
  (Development|PrintString (Utilities|String|Append "Ammo: " (Utilities|String|Append (Utilities|String|ToString(Integer) _output_get) (Utilities|String|Append " / " (Utilities|String|ToString(Integer) (Variables|/Game/Production/Blueprints/BP_FirstPersonShooterCharacter.BP_FirstPersonShooterCharacter_C|GetFullAmmo _asbp_first_person_shooter_character))))))
  (Utilities|FlowControl|Delay 3.0)
  (Rendering|SetActorHiddenInGame false)
  (Collision|SetActorEnableCollision true))

(fn ConstructionScript)